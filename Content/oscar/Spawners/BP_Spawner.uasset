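; BP_Spawner is an actor that spawns a limited number of BP_Enemy actors at its own transform, one at a time.
; TriggerSpawn starts a looping timer at the configured spawn delay and stores its handle.
; Each tick of that timer spawns an enemy and decrements Count, and the first tick after Count runs out clears the timer.
; Nothing in this Blueprint calls TriggerSpawn.
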(event `TriggerSpawn`
  (bind _returnvalue (`KismetSystemLibrary.K2_SetTimerDelegate` (delegate `spawnenemy`) (`self.spawndelay`) true))
  (set `self.timerref` _returnvalue))

(event `spawnenemy`
  (if (> (`self.count`) 0)
    (`|SpawnActorFromClass` "/Game/oscar/character/BP_Enemy.BP_Enemy_C" (`self.GetTransform`) "Undefined" "MultiplyWithRoot" null null)
    (`/Engine/EditorBlueprintResources/StandardMacros.DecrementInt` (`self.count`))
    (else
      (`KismetSystemLibrary.K2_ClearAndInvalidateTimerHandle` (`self.timerref`)))))

(fn `UserConstructionScript`)