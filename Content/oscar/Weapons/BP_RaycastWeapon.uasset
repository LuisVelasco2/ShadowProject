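; Raycast weapon Blueprint that fires one hitscan shot per StartFire call while ammo remains, through a gate that StopFire closes.
; Each shot traces from the Muzzle socket along its forward vector up to Range, with debug drawing, and applies damage to the hit actor.
; It also decrements ammo, plays sound and the owner's montage, and spawns a bullet actor aimed at the trace result.
; The muzzle emitter is unconnected.
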(event `self.StartFire`
  (bind (_startpoint _endpoint) (`self.startandendpoint`))
  (`|ExecutionSequence`
    (:`then_0`
      (goto _label :!via `Open`))
    (:`then_1`
      (`/Engine/EditorBlueprintResources/StandardMacros.Gate` true :!label _label
        (:`Exit`
          (if (> (`self.ammo`) 0)
            (bind _outhit (`KismetSystemLibrary.LineTraceSingle` _startpoint _endpoint "TraceTypeQuery3" false (`|MakeArray` (`self.OwnerReference`) :!type "Actor Object Reference") "ForDuration" true (struct :`R` 1.0 :`A` 1.0) (struct :`G` 1.0 :`A` 1.0) 1.0))
            (`self.DecrementAmmo`)
            (bind (_bblockinghit _binitialoverlap _time _distance _location _impactpoint _normal _impactnormal _physmat _hitactor _hitcomponent _hitbonename _bonename _hititem _elementindex _faceindex _tracestart _traceend) (`GameplayStatics.BreakHitResult` _outhit))
            (`self.PlayFX` _impactpoint (select `bool` _bblockinghit :`false` _traceend :`true` _impactpoint))
            (`GameplayStatics.ApplyDamage` _hitactor (`self.Damage`) null (`self.OwnerReference`))))))))

(event `self.StopFire`
  (goto _label :!via `Close`))

(fn `DecrementAmmo`
  (`/Engine/EditorBlueprintResources/StandardMacros.DecrementInt` (`self.ammo`)
    (:`  `
      (return))))

(fn `PlayFX`
  (params (impactpoint :type "Vector Structure") (`trace end` :type "Vector Structure"))
  (bind _muzzleposition (`self.Muzzleposition`))
  (`GameplayStatics.PlaySoundAtLocation` "/Game/oscar/Sounds/Player/shoot.shoot" (`self.Muzzleposition`) (struct) 1.0 1.0 0.0 null null null null)
  (`Character.PlayAnimMontage` (`self.OwnerReference`) "/Game/oscar/character/Animations/Player/AM_SHOOT.AM_SHOOT" 1.0 "None")
  (`|SpawnActorFromClass` "/Game/oscar/Weapons/BP_ProyectalBullets.BP_ProyectalBullets_C" (`KismetMathLibrary.MakeTransform` _muzzleposition (`KismetMathLibrary.FindLookAtRotation` _muzzleposition (`local.trace end`))) "Undefined" "MultiplyWithRoot" null null))

(fn `startandendpoint`
  (returns (startPoint :type "Vector Structure") (EndPoint :type "Vector Structure"))
  (bind _skeletalmesh (`self.SkeletalMesh`))
  (bind _output_get (set `self.Muzzleposition` (`SceneComponent.GetSocketLocation` _skeletalmesh "Muzzle")))
  (return _output_get (+ _output_get (* (`KismetMathLibrary.GetForwardVector` (`SceneComponent.GetSocketRotation` _skeletalmesh "Muzzle")) (`self.range`)))))

(fn `UserConstructionScript`
  (`parent.UserConstructionScript`))